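; BP_PlayerPs1 drives a scene capture camera and keeps the material on a referenced TV mesh informed of that camera's position.
; The construction script assigns the TextureTarget variable as the SceneCaptureComponent2D's render target.
; BeginPlay replaces the TV mesh's second material slot with a dynamic instance.
; Each Tick writes the capture component's world location into that instance's RenderTextureCamera vector parameter.
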(event EventBeginPlay
  (bind _tv (Variables|Default|GetTV))
  (bind _staticmeshcomponent (Variables|/Script/Engine.StaticMeshActor|GetStaticMeshComponent _tv))
  (bind _returnvalue (Rendering|Material|CreateDynamicMaterialInstance _staticmeshcomponent 1 (Rendering|Material|GetMaterial _staticmeshcomponent 1) "None" :!class /Script/Engine.PrimitiveComponent))
  (bind _output_get (Variables|Default|SetTVMaterial _returnvalue))
  (Rendering|Material|SetMaterial (Variables|/Script/Engine.StaticMeshActor|GetStaticMeshComponent (Variables|Default|GetTV)) 1 _output_get))

(event Collision|EventActorBeginOverlap
  (params (OtherActor :type Actor%20Object%20Reference)))

(event EventTick
  (params (DeltaSeconds :type Float%20%28single-precision%29))
  (Rendering|Material|SetVectorParameterValue (Variables|Default|GetTVMaterial) "RenderTextureCamera" (Math|Conversions|ToLinearColor(Vector) (Transformation|GetWorldLocation (Variables|Default|GetSceneCaptureComponent2D))) :!class /Script/Engine.MaterialInstanceDynamic))

(fn ConstructionScript
  (Variables|/Script/Engine.SceneCaptureComponent2D|SetTextureTarget (Variables|Default|GetSceneCaptureComponent2D) (Variables|Default|GetTexture%20Target)))