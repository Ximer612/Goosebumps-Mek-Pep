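; Actor component that plays surface-dependent footstep sounds for its owner.
; It creates an audio component with the footstep cue on BeginPlay, and ShouldPlayFootstep triggers a step once the owner is far enough from the last foot position while moving on ground.
; With zero vertical velocity, a downward line trace records that position and maps the hit physical material's index in Surfaces to the cue's Surface parameter before playback.
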(event Custom|ShouldPlayFootstep
  (bind _returnvalue (Components|GetOwner))
  (if (and (> (Math|Vector|VectorLength (- (Transformation|GetActorLocation _returnvalue) (Variables|Default|GetLastFootPosition))) (Variables|Default|GetFootstepSoundInterval)) (AI|Components|NavMovement|IsMovingonGround (Pawn|GetMovementComponent (Variables|/Script/Engine.Actor|GetInstigator _returnvalue))))
    (CallFunction|PlayFootstep)))

(event EventBeginPlay
  (bind _returnvalue (Game|AddComponentbyClass (Components|GetOwner) "/Script/Engine.AudioComponent" false))
  (bind _output_get (Variables|Default|SetFootstepSound _returnvalue))
  (Audio|Components|Audio|SetSound _output_get "/Game/Audio/Footstep/CUEs/CUE_FootSteps.CUE_FootSteps"))

(fn SurfaceDetect
  (bind _returnvalue (Components|GetOwner))
  (bind _returnvalue_2 (Transformation|GetActorLocation _returnvalue))
  (bind _outhit (Collision|LineTraceByChannel _returnvalue_2 (- _returnvalue_2 "0, 0,100.000000") "TraceTypeQuery1" false 0 "None"))
  (Variables|Default|SetLastFootPosition (.Location (Collision|BreakHitResult _outhit)))
  (bind (_array_element _array_index) (Utilities|Array|ForEachLoopwithBreak (Variables|Default|GetSurfaces) :!label _label)
    (:LoopBody
      (if (== _array_element (.PhysMat (Collision|BreakHitResult _outhit)))
        (Effects|Components|ParticleSystem|SetIntParameter (Variables|Default|GetFootstepSound) "Surface" _array_index)
        (goto _label Break)))))

(fn PlayFootstep
  ;[1 1 1] Is jumping?
  (if (== (.z (Transformation|GetVelocity (Components|GetOwner))) 0.0)
    (CallFunction|SurfaceDetect)
    (Audio|Components|Audio|Play (Variables|Default|GetFootstepSound) 0.0)))