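; Parent Blueprint for inspectable scene interactions that move the player's view to the object's own camera and back.
; Interact switches input context, fades, blends view and zooms slightly via timeline; IA_Drop reverses it.
; While inspecting, cursor traces swap to a lens over tagged points of interest, and clicks check any required inventory item, playing subtitles.
; Empty functions serve as child hooks for clicks and already-collected key items, checked on BeginPlay.
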(event Custom|OnSceneInteractionCompleted
  ;[0 1 0.2041] OnSceneInteractionCompleted
  (Input|DisableInput (Game|GetPlayerController 0)))

(event Custom|BackToPlayerCamera
  (bind _startcameralocation (Variables|Default|GetStartCameraLocation))
  (CallFunction|BeforeBacktoPlayer)
  (Input|DisableInput (Game|GetPlayerController 0))
  ;[1 1 1] camera back  to player's one
  (Collision|SetCollisionEnabled (Variables|Default|GetMouseInteractionTrigger) "NoCollision")
  (Collision|SetCollisionEnabled (Variables|Default|GetInteractionBox) "QueryOnly")
  (Variables|/Script/Engine.PlayerController|SetbShowMouseCursor (Game|GetPlayerController 0) false)
  (Variables|Default|SetIsMouseLeftClicked? false)
  (Variables|Default|SetIsMouseColliding? false)
  (CameraFades|StartCameraFade :self (Game|GetPlayerCameraManager 0) :ToAlpha 1.0 :Duration (* (Variables|Default|GetCameraHalfFade) 2.0))
  (bind _alpha (Timeline|TL_ZoomOut PlayFromStart)
    (:Update
      (Transformation|SetWorldLocation (Variables|Default|GetCamera) (Math|Vector|Lerp(Vector) (+ _startcameralocation (* (Math|Vector|GetForwardVector (Variables|Default|GetCamera)) 1e+01)) _startcameralocation _alpha) false true))
    (:Finished
      (Game|Player|SetViewTargetwithBlend (Game|GetPlayerController 0) (Game|Player|GetPlayerPawn 0) 0.0 "VTBlend_Linear" 0.0 false)
      (CameraFades|StartCameraFade :self (Game|GetPlayerCameraManager 0) :FromAlpha 1.0 :Duration (Variables|Default|GetCameraHalfFade))
      (Class|IPlayerUtils|SwitchInputContext(Message) (Game|Player|GetPlayerPawn 0) "/Game/Inputs/IMC_FirstPersonPlayer.IMC_FirstPersonPlayer" false)
      (Input|EnableInput (Game|Player|GetPlayerPawn 0) 0))))

(event Input|EnhancedActionEvents|EnhancedInputActionIA_Drop
  (params (ActionValue :type Boolean) (ElapsedSeconds :type Float%20%28double-precision%29) (TriggeredSeconds :type Float%20%28double-precision%29) (InputAction :type Input%20Action%20Object%20Reference :default "/Game/Inputs/Actions/IA_Drop.IA_Drop"))
  ;[1 1 1] On player interaction with this object change player camera to this object's camera
  (:Started
    (CallFunction|BacktoPlayerCamera)))

(event Input|EnhancedActionEvents|EnhancedInputActionIA_Interact
  (params (ActionValue :type Boolean) (ElapsedSeconds :type Float%20%28double-precision%29) (TriggeredSeconds :type Float%20%28double-precision%29) (InputAction :type Input%20Action%20Object%20Reference :default "/Game/Inputs/Actions/IA_Interact.IA_Interact"))
  (bind _returnvalue (Game|GetPlayerController 0))
  (bind _returnvalue_2 (Viewport|GetViewportSize))
  (bind _returnvalue_3 (Game|GetPlayerController 0))
  (bind _preinspectmouseposition (Variables|Default|GetPreInspectMousePosition))
  (bind _returnvalue_4 (* _returnvalue_2 "(X=0.500000,Y=0.500000)"))
  ;[1 0.2083 0.2182] ON INTERACT
  (:Triggered
    (if (not (Variables|/Script/Engine.PlayerController|GetbShowMouseCursor _returnvalue_3))
      (Class|PlayerController|SetMouseLocation _returnvalue_3 (Math|Float|Truncate (.x _returnvalue_4)) (Math|Float|Truncate (.y _returnvalue_4)))))
  (:Started
    (Variables|Default|SetIsMouseLeftClicked? true)
    (CallFunction|CheckifMouseonInteractionTrigger))
  (:Canceled
    (Variables|Default|SetIsMouseLeftClicked? false :!label _label)
    (if (Variables|Default|GetIsMouseColliding?)
      (Variables|Default|SetIsMouseColliding? false)
      (Class|PlayerController|SetMouseLocation _returnvalue (Math|Float|Truncate (.x _preinspectmouseposition)) (Math|Float|Truncate (.y _preinspectmouseposition)))
      (Variables|/Script/Engine.PlayerController|SetbShowMouseCursor _returnvalue true)))
  (:Completed
    (goto _label)))

(event EventBeginPlay
  ;[1 1 1] Begin Play
  (Variables|Default|SetStartCameraLocation (Transformation|GetWorldLocation (Variables|Default|GetCamera)))
  (bind _saveddata (Class|ISaveGame|GetGameData(Message) (Game|GetGameInstance)))
  (if (Utilities|Array|ContainsItem (.itemstaken (Variables|/Game/Blueprint/SaveGame/BP_GameData.BP_GameData_C|GetInventoryDiaryData _saveddata)) (Variables|Default|GetUnlockableItemRowName))
    (CallFunction|OnKeyItemAlreadyGot)))

(event EventSetSubtitlesManagerRef
  (params (SubtitleManagerRef :type BP%20Subtitles%20Manager%20Object%20Reference))
  (Variables|Default|SetSubtitle%20Manager%20Ref SubtitleManagerRef))

(event EventInteract
  (params (LookingComponent :type Primitive%20Component%20Object%20Reference))
  (bind _returnvalue (Game|Player|GetPlayerPawn 0))
  (bind _startcameralocation (Variables|Default|GetStartCameraLocation))
  ;[1 1 1] On player interaction with this object change player camera to this object's camera
  (Class|IPlayerUtils|SwitchInputContext(Message) _returnvalue "/Game/Inputs/IMC_Inspect.IMC_Inspect" true)
  (Collision|SetCollisionEnabled (Variables|Default|GetInteractionBox) "NoCollision")
  (Input|DisableInput _returnvalue (Game|GetPlayerController 0))
  (CameraFades|StartCameraFade :self (Game|GetPlayerCameraManager 0) :ToAlpha 1.0 :Duration (Variables|Default|GetCameraHalfFade))
  (Utilities|FlowControl|Delay (Variables|Default|GetCameraHalfFade))
  (Game|Player|SetViewTargetwithBlend (Game|GetPlayerController 0) self 0.0 "VTBlend_Linear" 0.0 false)
  (CameraFades|StartCameraFade :self (Game|GetPlayerCameraManager 0) :FromAlpha 1.0 :Duration (Variables|Default|GetCameraHalfFade))
  (bind _alpha (Timeline|TL_ZoomInALittleBit PlayFromStart)
    (:Update
      (Transformation|SetWorldLocation (Variables|Default|GetCamera) (Math|Vector|Lerp(Vector) _startcameralocation (+ _startcameralocation (* (Math|Vector|GetForwardVector (Variables|Default|GetCamera)) 1e+01)) _alpha) false true))
    (:Finished
      (Variables|/Script/Engine.PlayerController|SetbShowMouseCursor (Game|GetPlayerController 0) true)
      (Collision|SetCollisionEnabled (Variables|Default|GetMouseInteractionTrigger) "QueryAndPhysics")
      (Input|EnableInput (Game|GetPlayerController 0))
      (Actor|Tick|SetActorTickEnabled true)
      (Input|SetInputModeGameandUI (Game|GetPlayerController 0) 0 "DoNotLock" false true))))

(event EventTick
  (params (DeltaSeconds :type Float%20%28single-precision%29))
  (CallFunction|SetCursorInspection))

(fn ConstructionScript)

(fn OnKeyItemAlreadyGot)

(fn CheckifMouseonInteractionTrigger
  (bind _returnvalue (Game|GetPlayerController 0))
  (bind _returnvalue_2 (Game|GetPlayerController 0))
  (bind _hitresult (Game|Player|GetHitResultUnderCursorbyChannel _returnvalue "TraceTypeQuery3" false))
  (bind (_locationx _locationy) (Game|Player|GetMousePosition _returnvalue_2))
  (Utilities|IsValid (.hitcomponent _hitresult)
    (:Is%20Valid
      (if (and (.bblockinghit _hitresult) (Components|ComponentHasTag (.hitcomponent _hitresult) "ScenePointOfInterestTrigger"))
        (Variables|Default|SetIsMouseColliding? true)
        (Variables|Default|SetPreInspectMousePosition (Math|Vector2D|MakeVector2D _locationx _locationy))
        (Variables|/Script/Engine.PlayerController|SetbShowMouseCursor _returnvalue_2 false)
        (if (== (Variables|Default|GetToUseItemRowName) "")
          (CallFunction|OnClickonMouseInteractionTrigger :!label _label)
          (else
            (bind _hasitem_ (Class|IPlayerUtils|PlayerHasItem?(Message) (Game|Player|GetPlayerPawn 0) (Variables|Default|GetToUseItemRowName)))
            (if _hasitem_
              (Default|AddDialoguetoPlay (Variables|Default|GetSubtitle%20Manager%20Ref) (Variables|Default|GetDialogueRowNameOnUseKeyItem))
              (goto _label)
              (else
                (Default|AddDialoguetoPlay (Variables|Default|GetSubtitle%20Manager%20Ref) (Variables|Default|GetDialogueRowNameOnNoToUseKeyItem))))))
        (else
          (Variables|Default|SetIsMouseLeftClicked? false :!label _label_2))))
    (:Is%20Not%20Valid
      (goto _label_2))))

(fn OnClickonMouseInteractionTrigger)

(fn BeforeBacktoPlayer
  (Input|SetInputModeGameOnly (Game|GetPlayerController 0) true)
  (Actor|Tick|SetActorTickEnabled false))

(fn SetCursorInspection
  (bind _returnvalue (Game|GetPlayerController 0))
  (bind _hitresult (Game|Player|GetHitResultUnderCursorbyChannel _returnvalue "TraceTypeQuery3" true))
  (Utilities|IsValid (.hitcomponent _hitresult)
    (:Is%20Valid
      (if (and (.bblockinghit _hitresult) (Components|ComponentHasTag (.hitcomponent _hitresult) "ScenePointOfInterestTrigger"))
        (Class|WidgetBlueprintLibrary|SetHardwareCursor "Default" "T_CursorLens" "(X=0.200000,Y=0.200000)")
        (else
          (Class|WidgetBlueprintLibrary|SetHardwareCursor "Default" "T_Cursor" "(X=0.500000,Y=0.500000)" :!label _label))))
    (:Is%20Not%20Valid
      (goto _label))))